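; Lobby game mode for a multiplayer room: tracks players, handles ready updates and kicks, and starts the match.
; On login it spawns and possesses a BP_MyCharacter at the first PlayerStart found; logout removes the player from parallel controller and info lists.
; Logout and ready changes push the list, plus room settings from the GameInstance, to each BP_LobbyController.
; Starting shows loading UI on every controller, then ServerTravels to MyMap.
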(event `self.K2_OnLogout`
  (params (ExitingController :type "Controller Object Reference"))
  ;[1 1 1] 玩家登出
  (for (_array_element _array_index) (`self.PlayerList`)
    (if (== _array_element ExitingController)
      (`KismetArrayLibrary.Array_RemoveItem` (`self.PlayerList`) _array_element)
      (`KismetArrayLibrary.Array_Remove` (`self.PlayerInfoList`) _array_index)))
  (`self.EVE_UpdateAllPlayer`))

(event `self.K2_PostLogin`
  (params (NewPlayer :type "PlayerController Object Reference"))
  ;[1 1 1] 玩家登录
  (`KismetArrayLibrary.Array_AddUnique` (`self.PlayerList`) NewPlayer)
  (`self.EVE_SpawnPlayer` NewPlayer))

(event `self.ReceiveBeginPlay`
  ;[1 1 1] 获取当前地图信息
  (bind _asbp_my_game_instance (cast `/Game/ShootingRange/Room/BP_MyGameInstance` (`GameplayStatics.GetGameInstance`)))
  (set `self.Room Name` (`/Game/ShootingRange/Room/BP_MyGameInstance.RoomName` _asbp_my_game_instance))
  (set `self.Room Max Person` (`/Game/ShootingRange/Room/BP_MyGameInstance.RoomMaxPlayer` _asbp_my_game_instance)))

(event `EVE_SpawnPlayer`
  (params (PlayerController :type "PlayerController Object Reference"))
  (bind _returnvalue (`Controller.K2_GetPawn` PlayerController))
  ;[1 1 1] 生成玩家
  (`/Engine/EditorBlueprintResources/StandardMacros.IsValid` _returnvalue
    (:`Is Valid`
      (`self.K2_DestroyActor` _returnvalue))
    (:`Is Not Valid`
      _))
  (bind _outactors (`GameplayStatics.GetAllActorsOfClass` "/Script/Engine.PlayerStart"))
  (bind _returnvalue_2 (`|SpawnActorFromClass` "/Game/ShootingRange/Blueprints/Character/BP_MyCharacter.BP_MyCharacter_C" (`KismetMathLibrary.MakeTransform` (`self.K2_GetActorLocation` (`|GetArrayItem` _outactors))) "AdjustIfPossibleButAlwaysSpawn" "OverrideRootScale" null null))
  (`Controller.Possess` PlayerController _returnvalue_2))

(event `EVE_UpdateAllPlayer`
  ;[1 1 1] 更新所有玩家
  (for _array_element (`self.PlayerList`)
    (bind _asbp_lobby_controller (cast `/Game/ShootingRange/Room/Lobby/BP_LobbyController` _array_element))
    (`/Game/ShootingRange/Room/Lobby/BP_LobbyController.EVE_UpdateSelf` _asbp_lobby_controller (`self.PlayerInfoList`) (`self.Room Name`) (`self.Room Max Person`))))

(event `EVE_AddPlayerInfo`
  (params (PlayerInfo :type "/Game/ShootingRange/Room/Variable/SPlayerInfo Structure (by ref)"))
  ;[1 1 1] 添加玩家信息
  (`KismetArrayLibrary.Array_Add` (`self.PlayerInfoList`) PlayerInfo))

(event `EVE_UpdateReadyInfo`
  (params (PlayerInfoList :type "/Game/ShootingRange/Room/Variable/SPlayerInfo Structure"))
  (bind _newplayerinfolist (`self.NewPlayerInfoList`))
  ;[1 1 1] 更新准备信息
  (`KismetArrayLibrary.Array_Clear` (`self.NewPlayerInfoList`))
  (for _array_element (`self.PlayerInfoList`)
    (if (`KismetTextLibrary.EqualEqual_TextText` (`.Name_3_1AD422A249143FCB9A314A9DBD8897D1` (break `/Game/ShootingRange/Room/Variable/SPlayerInfo` _array_element)) (`.Name_3_1AD422A249143FCB9A314A9DBD8897D1` (break `/Game/ShootingRange/Room/Variable/SPlayerInfo` PlayerInfoList)))
      (`KismetArrayLibrary.Array_Add` _newplayerinfolist PlayerInfoList)
      (else
        (`KismetArrayLibrary.Array_Add` _newplayerinfolist _array_element))))
  (set `self.PlayerInfoList` (`self.NewPlayerInfoList`))
  (`KismetArrayLibrary.Array_Clear` (`self.NewPlayerInfoList`))
  (`self.EVE_UpdateAllPlayer`))

(event `EVE_KickPlayer`
  (params (PlayerIndex :type Integer))
  ;[1 1 1] 踢出房间
  (bind _asbp_lobby_controller (cast `/Game/ShootingRange/Room/Lobby/BP_LobbyController` (`|GetArrayItem` (`self.PlayerList`) PlayerIndex)))
  (`/Game/ShootingRange/Room/Lobby/BP_LobbyController.EVE_LeaveRoom` _asbp_lobby_controller))

(event `EVE_StartGame`
  ;[1 1 1] 服务器将开始游戏的信息传给客户端
  (for _array_element (`self.PlayerList`)
    (bind _asbp_lobby_controller (cast `/Game/ShootingRange/Room/Lobby/BP_LobbyController` _array_element))
    (`/Game/ShootingRange/Room/Lobby/BP_LobbyController.EVE_CreateLoadingUI` _asbp_lobby_controller _asbp_lobby_controller))
  (`self.EVE_JumpToMap`))

(event `EVE_JumpToMap`
  ;[1 1 1] 跳到指定关卡
  (`KismetSystemLibrary.ExecuteConsoleCommand` "ServerTravel  MyMap" (`GameplayStatics.GetPlayerController` 0)))

(fn `UserConstructionScript`)