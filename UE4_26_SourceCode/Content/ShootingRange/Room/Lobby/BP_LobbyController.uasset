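; Player controller for the shooting range's multiplayer room lobby, linking each player's lobby UI to BP_LobbyGameMode.
; On BeginPlay it registers PlayerInfo from the game instance, shows WBP_Lobby and announces the join in chat.
; It forwards player updates, kicks and game start to the game mode, and relays chat through every controller in its PlayerList.
; It also receives UI refreshes, creates the loading screen and destroys the session to return to Map_Start.
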(event `self.ReceiveBeginPlay`
  (`self.EVE_Init`))

(event `EVE_Init`
  ;[1 1 1] 初始化玩家信息
  (bind _asbp_my_game_instance (cast `/Game/ShootingRange/Room/BP_MyGameInstance` (`GameplayStatics.GetGameInstance`)))
  (bind _output_get (set `self.PlayerInfo` (`/Game/ShootingRange/Room/BP_MyGameInstance.PlayerInfo` _asbp_my_game_instance)))
  (bind (_name _serverclient) (break `/Game/ShootingRange/Room/Variable/SPlayerInfo` _output_get))
  (`KismetSystemLibrary.PrintString` (`KismetTextLibrary.Conv_TextToString` _name))
  (`KismetSystemLibrary.PrintString` (`KismetTextLibrary.Conv_TextToString` _serverclient))
  (`self.EVE_AddPlayerInfo` (`self.PlayerInfo`))
  (`self.EVE_ShowLobbyUI`))

(event `EVE_ShowLobbyUI`
  (bind _playerinfo_name (break `/Game/ShootingRange/Room/Variable/SPlayerInfo` (`self.PlayerInfo`)))
  ;[1 1 1] 创建显示大厅
  (set `self.bShowMouseCursor` true)
  (bind _returnvalue (`|CreateWidget` "/Game/ShootingRange/Room/UI/WBP_Lobby.WBP_Lobby_C" self))
  (bind _output_get (set `self.LobbyUI` _returnvalue))
  (`UserWidget.AddToViewport` _output_get 0)
  (`self.EVE_UpdateAllPlayer`)
  (`self.EVE_AddChatInfo` "【系统】" (`|FormatText` "玩家 {name} 进入房间" _playerinfo_name)))

(event `EVE_UpdateAllPlayer`
  ;[1 1 1] 更新所有玩家
  (bind _asbp_lobby_game_mode (cast `/Game/ShootingRange/Room/Lobby/BP_LobbyGameMode` (`GameplayStatics.GetGameMode`)))
  (`/Game/ShootingRange/Room/Lobby/BP_LobbyGameMode.EVE_UpdateAllPlayer` _asbp_lobby_game_mode))

(event `EVE_AddPlayerInfo`
  (params (PlayerInfo :type "/Game/ShootingRange/Room/Variable/SPlayerInfo Structure (by ref)"))
  ;[1 1 1] 为GameMode添加玩家信息
  (bind _asbp_lobby_game_mode (cast `/Game/ShootingRange/Room/Lobby/BP_LobbyGameMode` (`GameplayStatics.GetGameMode`)))
  (`/Game/ShootingRange/Room/Lobby/BP_LobbyGameMode.EVE_AddPlayerInfo` _asbp_lobby_game_mode PlayerInfo))

(event `EVE_UpdateSelf`
  (params (PlayerInfo :type "Array of /Game/ShootingRange/Room/Variable/SPlayerInfo Structure") (RoomName :type Text) (RoomMaxPerson :type Integer))
  ;[1 1 1] 更新自身大厅UI信息
  (`/Game/ShootingRange/Room/UI/WBP_Lobby.EVE_UpdateInfo` (`self.LobbyUI`) PlayerInfo RoomName RoomMaxPerson))

(event `EVE_UpdatePlayerInfo`
  (params (PlayerInfoList :type "/Game/ShootingRange/Room/Variable/SPlayerInfo Structure"))
  ;[1 1 1] 更新玩家信息
  (bind _asbp_lobby_game_mode (cast `/Game/ShootingRange/Room/Lobby/BP_LobbyGameMode` (`GameplayStatics.GetGameMode`)))
  (`/Game/ShootingRange/Room/Lobby/BP_LobbyGameMode.EVE_UpdateReadyInfo` _asbp_lobby_game_mode PlayerInfoList))

(event `EVE_LeaveRoom`
  ;[1 1 1] 离开房间
  (`DestroySessionCallbackProxy.DestroySession` self
    (:`OnSuccess`
      (`KismetSystemLibrary.PrintString` "Leave successed")
      (`GameplayStatics.OpenLevel` "Map_Start"))
    (:`OnFailure`
      (`KismetSystemLibrary.PrintString` "Leave failed"))))

(event `EVE_KickPlayer`
  (params (PlayerIndex :type Integer))
  (bind _asbp_lobby_game_mode (cast `/Game/ShootingRange/Room/Lobby/BP_LobbyGameMode` (`GameplayStatics.GetGameMode`)))
  (`/Game/ShootingRange/Room/Lobby/BP_LobbyGameMode.EVE_KickPlayer` _asbp_lobby_game_mode PlayerIndex))

(event `EVE_NewMessage`
  (params (Text :type Text))
  ;[1 1 1] 更新新的消息
  (`/Game/ShootingRange/Room/UI/WBP_ChatFrame.EVE_UpdateNewMessage` (`/Game/ShootingRange/Room/UI/WBP_Lobby.WBP_ChatFrame` (`self.LobbyUI`)) Text))

(event `EVE_AddChatInfo`
  (params (Speaker :type Text) (text :type Text))
  ;[1 1 1] 增加新信息
  (bind _asbp_lobby_game_mode (cast `/Game/ShootingRange/Room/Lobby/BP_LobbyGameMode` (`GameplayStatics.GetGameMode`)))
  (for _array_element (`/Game/ShootingRange/Room/Lobby/BP_LobbyGameMode.PlayerList` _asbp_lobby_game_mode)
    (bind _asbp_lobby_controller (cast `/Game/ShootingRange/Room/Lobby/BP_LobbyController` _array_element))
    (`self.EVE_NewMessage` _asbp_lobby_controller (`|FormatText` "{speaker}：{text}" Speaker text))))

(event `EVE_StartGame`
  ;[1 1 1] 开始游戏传给服务器
  (bind _asbp_lobby_game_mode (cast `/Game/ShootingRange/Room/Lobby/BP_LobbyGameMode` (`GameplayStatics.GetGameMode`)))
  (`/Game/ShootingRange/Room/Lobby/BP_LobbyGameMode.EVE_StartGame` _asbp_lobby_game_mode))

(event `EVE_CreateLoadingUI`
  (params (OwningPlayer :type "PlayerController Object Reference"))
  ;[1 1 1] 创建加载界面
  (bind _returnvalue (`|CreateWidget` "/Game/ShootingRange/Room/UI/WBP_Loading.WBP_Loading_C" OwningPlayer))
  (`UserWidget.AddToViewport` _returnvalue 0))

(fn `UserConstructionScript`)