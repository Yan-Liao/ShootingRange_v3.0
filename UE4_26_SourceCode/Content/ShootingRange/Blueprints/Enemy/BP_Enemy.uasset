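; Networked AI enemy character for the shooting range that patrols, senses players, fights with a holstered weapon and can flee.
; PawnSensing, patrol and damage events write to the blackboard, while exposed events handle equipping, aiming, firing and reloading.
; Damage updates the health bar, may trigger a random retreat at low HP, and at zero ragdolls and notifies GameState.
; Tick computes aim, movement and left-hand grip IK values, returned by EnemySendValue.
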(event `self.ReceiveBeginPlay`
  (`self.Enemy_Init`))

(event `self.ReceiveTick`
  (params (DeltaSeconds :type "Float (single-precision)"))
  ;[1 1 1] Tick
  (`self.ROS_EnemyTick`))

(event `ROS_EnemyTick`
  (bind _returnvalue (`self.GetVelocity`))
  (bind (_returnvalue_roll _returnvalue_pitch _returnvalue_yaw) (`KismetMathLibrary.BreakRotator` (`KismetMathLibrary.NormalizedDeltaRotator` (`self.GetBaseAimRotation`) (`self.K2_GetActorRotation`))))
  ;[1 1 1] Tick
  (set `self.IsInAir` (`NavMovementComponent.IsFalling` (`self.CharacterMovement`)))
  (set `self.Speed` (`KismetMathLibrary.VSize` _returnvalue))
  (set `self.Dirction` (`AnimInstance.CalculateDirection` (`SkeletalMeshComponent.GetAnimInstance` (`self.Mesh`)) _returnvalue (`self.K2_GetActorRotation`)))
  (set `self.Pitch` _returnvalue_pitch)
  (set `self.Yaw` _returnvalue_yaw)
  (`self.ToggleHandL IK`)
  (`self.CaculateLHandOfset`))

(event `/Game/ShootingRange/Blueprints/Enemy/BPI_Enemy.EnemyGetWeapon`
  (params (WeaponActor :type "Actor Object Reference"))
  (bind _mesh (`self.Mesh`))
  ;[1 1 1] GetWeapon
  (bind _asbp_weapon_base (cast `/Game/ShootingRange/Blueprints/Weapons/BP_WeaponBase` WeaponActor))
  (message `/Game/ShootingRange/Blueprints/Weapons/BPI_WeaponBase.GetWeapon` WeaponActor self)
  (bind _skeletalmesh (`/Game/ShootingRange/Blueprints/Weapons/BP_WeaponBase.SkeletalMesh` _asbp_weapon_base))
  (`PrimitiveComponent.SetSimulatePhysics` _skeletalmesh false)
  (`PrimitiveComponent.SetCollisionResponseToChannel` _skeletalmesh "ECC_GameTraceChannel1" "ECR_Ignore")
  (bind _weapontype (`/Game/ShootingRange/Blueprints/Weapons/BP_WeaponBase.WeaponType` _asbp_weapon_base))
  (set `self.Weapon Type` _weapontype)
  (if (`|EnumEquality` _weapontype "NewEnumerator0")
    (`self.K2_AttachToComponent` WeaponActor _mesh "HolsterBRSocket" "SnapToTarget" "SnapToTarget" "SnapToTarget" true)
    (set `self.WeaponSlot` (make `/Game/ShootingRange/Blueprints/Weapons/SWeaponSlot` _asbp_weapon_base "NewEnumerator0" "HolsterBRSocket"))
    (else
      (`self.K2_AttachToComponent` WeaponActor _mesh "HolsterThighRSocket" "SnapToTarget" "SnapToTarget" "SnapToTarget" true)
      (set `self.WeaponSlot` (make `/Game/ShootingRange/Blueprints/Weapons/SWeaponSlot` _asbp_weapon_base "NewEnumerator1" "HolsterThighRSocket")))))

(event `ROM_EquipHolsterWeaponMontage`
  (params (InSkeletalMeshComponent :type "SkeletalMeshComponent Object Reference") (MontageToPlay :type "AnimMontage Object Reference"))
  ;[1 1 1] EquipHolsterWeapon
  (`|PlayMontage` InSkeletalMeshComponent MontageToPlay))

(event `ROS_EquipWeapon`
  (bind _equipmontage (`self.EquipMontage`))
  ;[1 1 1] EquipHolsterWeapon
  (set `self.IsCombate` true)
  (`self.ROM_EquipHolsterWeaponMontage` (`self.Mesh`) (select `bool` (`|EnumEquality` (`self.Weapon Type`) "NewEnumerator0") :`false` (`|GetArrayItem` _equipmontage) :`true` (`|GetArrayItem` _equipmontage 1))))

(event `GrabWeaponBLTemp`
  (bind _weaponslot_weaponbase (break `/Game/ShootingRange/Blueprints/Weapons/SWeaponSlot` (`self.WeaponSlot`)))
  ;[1 1 1] EquipHolsterWeapon
  (`self.ROS_GrabWeaponBLTemp` _weaponslot_weaponbase (`self.Mesh`)))

(event `EquipWeaponBR`
  (bind _weaponslot_weaponbase (break `/Game/ShootingRange/Blueprints/Weapons/SWeaponSlot` (`self.WeaponSlot`)))
  ;[1 1 1] EquipHolsterWeapon
  (`self.ROS_EquipWeaponBR` _weaponslot_weaponbase (`self.Mesh`)))

(event `HolsterWeaponBR`
  (bind (_weaponslot_weaponbase _weaponslot_weapontype _weaponslot_holster) (break `/Game/ShootingRange/Blueprints/Weapons/SWeaponSlot` (`self.WeaponSlot`)))
  ;[1 1 1] EquipHolsterWeapon
  (`self.ROS_HolsterWeaponBR` _weaponslot_weaponbase (`self.Mesh`) _weaponslot_holster))

(event `ROS_HolsterWeapon`
  (bind _holstermontage (`self.HolsterMontage`))
  ;[1 1 1] EquipHolsterWeapon
  (set `self.IsADS` false)
  (set `self.IsCombate` false)
  (`self.ROM_EquipHolsterWeaponMontage` (`self.Mesh`) (select `bool` (`|EnumEquality` (`self.Weapon Type`) "NewEnumerator0") :`false` (`|GetArrayItem` _holstermontage) :`true` (`|GetArrayItem` _holstermontage 1))))

(event `ROS_GrabWeaponBLTemp`
  (params (Weapon :type "Actor Object Reference") (Parent :type "SceneComponent Object Reference"))
  ;[1 1 1] EquipHolsterWeapon
  (`self.K2_AttachToComponent` Weapon Parent "HandLSocket" "SnapToTarget" "SnapToTarget" "SnapToTarget" true))

(event `ROS_EquipWeaponBR`
  (params (Weapon :type "Actor Object Reference") (Parent :type "SceneComponent Object Reference"))
  ;[1 1 1] EquipHolsterWeapon
  (`self.K2_AttachToComponent` Weapon Parent "HandRSocket" "SnapToTarget" "SnapToTarget" "SnapToTarget" true)
  (bind _asbp_weapon_base (cast `/Game/ShootingRange/Blueprints/Weapons/BP_WeaponBase` Weapon))
  (set `self.Aim Baseline Offset` (`/Game/ShootingRange/Blueprints/Weapons/BP_WeaponBase.AimBaselineOffset` _asbp_weapon_base)))

(event `ROS_HolsterWeaponBR`
  (params (Weapon :type "Actor Object Reference") (Parent :type "SceneComponent Object Reference") (SocketName :type Name))
  ;[1 1 1] EquipHolsterWeapon
  (`self.K2_AttachToComponent` Weapon Parent SocketName "SnapToTarget" "SnapToTarget" "SnapToTarget" true))

(event `ROS_Fire`
  (bind _weaponslot_weaponbase (break `/Game/ShootingRange/Blueprints/Weapons/SWeaponSlot` (`self.WeaponSlot`)))
  ;[1 1 1] Fire/ToggleFireMode
  (if (and (`self.IsCombate`) (not (`self.IsReloading`)))
    (`self.ROS_FireWeapon` _weaponslot_weaponbase)))

(event `ROS_FireWeapon`
  (params (`Weapon Base` :type "/Game/ShootingRange/Blueprints/Weapons/BP_WeaponBase Object Reference"))
  ;[1 1 1] Fire/ToggleFireMode
  (`/Game/ShootingRange/Blueprints/Weapons/BPI_WeaponBase.FireWeapon` `Weapon Base`))

(event `ROS_FireRelease`
  (params (`目标` :type "/Game/ShootingRange/Blueprints/Weapons/BP_WeaponBase Object Reference"))
  ;[1 1 1] Fire/ToggleFireMode
  (`/Game/ShootingRange/Blueprints/Weapons/BP_WeaponBase.FireRelease` `目标`))

(event `ROS_FinishFire`
  (bind _weaponslot_weaponbase (break `/Game/ShootingRange/Blueprints/Weapons/SWeaponSlot` (`self.WeaponSlot`)))
  ;[1 1 1] Fire/ToggleFireMode
  (if (and (`self.IsCombate`) (not (`self.IsReloading`)))
    (`self.ROS_FireRelease` _weaponslot_weaponbase)))

(event `ROS_Reload`
  (bind _weaponslot_weaponbase (break `/Game/ShootingRange/Blueprints/Weapons/SWeaponSlot` (`self.WeaponSlot`)))
  ;[1 1 1] Reload
  (if (`self.IsCombate`)
    (set `self.IsReloading` true)
    (`self.ROM_ReloadMontage` (`self.Mesh`) (`/Game/ShootingRange/Blueprints/Weapons/BP_WeaponBase.ReloadMontageChar` _weaponslot_weaponbase))
    (`|ExecutionSequence`
      (:`then_0`
        (`/Game/ShootingRange/Blueprints/Weapons/BP_WeaponBase.ReloadWeapon` _weaponslot_weaponbase))
      (:`then_1`
        (`KismetSystemLibrary.Delay` 1.5)
        (set `self.IsReloading` false)))))

(event `ROM_ReloadMontage`
  (params (InSkeletalMeshComponent :type "SkeletalMeshComponent Object Reference") (MontageToPlay :type "AnimMontage Object Reference"))
  ;[1 1 1] Reload
  (`|PlayMontage` InSkeletalMeshComponent MontageToPlay))

(event `ROS_GetDamage`
  (params (Damage :type "Float (double-precision)"))
  (bind _returnvalue (`AIBlueprintHelperLibrary.GetBlackboard` self))
  (bind _returnvalue_2 (`AIBlueprintHelperLibrary.GetBlackboard` self))
  ;[1 1 1] GotDamage
  (bind _output_get (set `self.hp` (`KismetMathLibrary.FMax` (- (`self.hp`) Damage))))
  (`|ExecutionSequence`
    (:`then_0`
      (`/Engine/EditorBlueprintResources/StandardMacros.CompareFloat` _output_get
        (:`==`
          _)
        (:`<`
          _))
      (`/Engine/EditorBlueprintResources/StandardMacros.DoOnce` false
        (:`Completed`
          (`self.ROM_EnemyDown`))))
    (:`then_1`
      (`/Engine/EditorBlueprintResources/StandardMacros.DoOnce` false
        (:`Completed`
          (if (== (`BlackboardComponent.GetValueAsObject` _returnvalue (`self.Player`)) null)
            (`BlackboardComponent.SetValueAsObject` _returnvalue (`self.Player`) (stale `self.ReceiveAnyDamage` DamageCauser))))))
    (:`then_2`
      (`/Engine/EditorBlueprintResources/StandardMacros.CompareFloat` _output_get (* (`self.MaxHp`) (`self.RunAwayPercent`))
        (:`==`
          _)
        (:`<`
          _))
      (`/Engine/EditorBlueprintResources/StandardMacros.DoOnce` false
        (:`Completed`
          (`/Engine/EditorBlueprintResources/StandardMacros.CompareFloat` (`KismetMathLibrary.RandomFloatInRange` 0.0 10.0) 5.0
            (:`<`
              (`KismetSystemLibrary.Delay` 1.0)
              (set `CharacterMovementComponent.MaxWalkSpeed` (`self.RunSpeed`) (`self.CharacterMovement`))
              (set `self.IsADS` false)
              (`/Engine/EditorBlueprintResources/StandardMacros.IsValid` _returnvalue_2
                (:`Is Valid`
                  (`BlackboardComponent.SetValueAsBool` _returnvalue_2 (`self.IsRunAway`) true))))))))
    (:`then_3`
      (`self.ROM_SetHpBar` (/ (`self.hp`) (`self.MaxHp`))))))

(event `self.ReceiveAnyDamage`
  (params (Damage :type "Float (single-precision)") (DamageType :type "DamageType Object Reference") (InstigatedBy :type "Controller Object Reference") (DamageCauser :type "Actor Object Reference"))
  ;[1 1 1] GotDamage
  (`self.ROS_GetDamage` Damage))

(event `ROM_EnemyDown`
  (bind _mesh (`self.Mesh`))
  ;[1 1 1] GotDamage
  (set `self.IsDown` true)
  (`self.DetachFromControllerPendingDestroy`)
  (`MovementComponent.StopMovementImmediately` (`self.CharacterMovement`))
  (`PrimitiveComponent.SetCollisionEnabled` _mesh "QueryAndPhysics")
  (`PrimitiveComponent.SetSimulatePhysics` _mesh true)
  (`self.SetLifeSpan` 2.0)
  (`self.LossWeapon`)
  (bind _asbp_my_game_state (cast `/Game/ShootingRange/Blueprints/BP_MyGameState` (`GameplayStatics.GetGameState`)))
  (`/Game/ShootingRange/Blueprints/BP_MyGameState.EnemyDown` _asbp_my_game_state))

(event `ROS_EnemyRun`
  ;[1 1 1] shift奔跑
  (`self.ROM_SetSpeed` (`self.RunSpeed`) (`self.CharacterMovement`)))

(event `ROM_SetSpeed`
  (params (`最大行走速度` :type "Float (double-precision)") (`目标` :type "CharacterMovementComponent Object Reference"))
  ;[1 1 1] shift奔跑
  (set `CharacterMovementComponent.MaxWalkSpeed` `最大行走速度` `目标`))

(event `ROS_EnemyWalk`
  ;[1 1 1] shift奔跑
  (`self.ROM_SetSpeed` (`self.WalkSpeed`) (`self.CharacterMovement`)))

(event `GetNextPoint`
  ;[1 1 1] GetPatrolPoint
  (if (`KismetSystemLibrary.IsServer`)
    (bind _nextitem (`/Game/ShootingRange/Blueprints/Character/BPML_MacroLibrary.GetArrayNextItem` (`self.PatrolPointsList`) (`self.CurrentPotrolPoint`))
      (:`Out`
        (bind _output_get (set `self.CurrentPotrolPoint` _nextitem))
        (`BlackboardComponent.SetValueAsObject` (`AIBlueprintHelperLibrary.GetBlackboard` self) (`self.PatrolPoint`) _output_get)))))

(event `SetBlackBoard`
  (bind _returnvalue (`AIBlueprintHelperLibrary.GetBlackboard` self))
  ;[1 1 1] 初始化设置黑板
  (`AIController.UseBlackboard` (`AIBlueprintHelperLibrary.GetAIController` self) "/Game/ShootingRange/Blueprints/Enemy/AI/BB_Enemy.BB_Enemy")
  (bind _output_get (set `self.CurrentPotrolPoint` (`|GetArrayItem` (`self.PatrolPointsList`))))
  (`BlackboardComponent.SetValueAsObject` _returnvalue (`self.PatrolPoint`) _output_get)
  (`BlackboardComponent.SetValueAsObject` _returnvalue (`self.SelfName`) self)
  (`BlackboardComponent.SetValueAsObject` _returnvalue (`self.RunAwayLocation`) (`self.RunAwayPlace`)))

(event `Enemy_Init`
  ;[1 1 1] EnemyInit
  (set `self.hp` (`self.MaxHp`))
  (`self.SetBlackBoard`)
  (bind _asbp_enemy_controler (cast `/Game/ShootingRange/Blueprints/Enemy/AI/BP_EnemyControler` (`self.GetController` self)))
  (`/Game/ShootingRange/Blueprints/Enemy/AI/BP_EnemyControler.EnemyComing` _asbp_enemy_controler))

(event `AttackPlayer`
  (params (Player :type "Actor Object Reference"))
  (bind _weaponslot_weaponbase (break `/Game/ShootingRange/Blueprints/Weapons/SWeaponSlot` (`self.WeaponSlot`)))
  ;[1 1 1] AttackPlayer
  (`self.FaceToPlayer` Player)
  (`/Engine/EditorBlueprintResources/StandardMacros.DoOnce` false :!label _label
    (:`Completed`
      (if (not (`self.IsCombate`))
        (`self.ROS_EquipWeapon`)
        (`KismetSystemLibrary.Delay` 1.5))
      (set `self.IsADS` true)
      (`/Engine/EditorBlueprintResources/StandardMacros.CompareInt` (`/Game/ShootingRange/Blueprints/Weapons/BP_WeaponBase.RoundsInChamber` _weaponslot_weaponbase)
        (:`>`
          _)
        (:`==`
          (`self.ROS_Reload` :!label _label_2))
        (:`<`
          (goto _label_2)))
      (`self.ROS_Fire`)
      (`/Engine/EditorBlueprintResources/StandardMacros.CompareFloat` (`KismetMathLibrary.Vector_Distance` (`self.K2_GetActorLocation` Player) (`self.K2_GetActorLocation`)) (`PawnSensingComponent.SightRadius` (`self.PawnSensing`))
        (:`>`
          (`BlackboardComponent.SetValueAsObject` (`AIBlueprintHelperLibrary.GetBlackboard` self) (`self.Player`) null))
        (:`==`
          _)
        (:`<`
          _))
      (`KismetSystemLibrary.Delay` 1.0)
      (goto _label :!via `Reset`))))

(event `self.PawnSensing.OnHearNoise`
  (params (Instigator :type "Pawn Object Reference") (Location :type "Vector Structure (by ref)") (Volume :type "Float (single-precision)"))
  (bind _returnvalue (`AIBlueprintHelperLibrary.GetBlackboard` self))
  ;[1 1 1] HearPlayer
  (if (`KismetSystemLibrary.IsServer`)
    (if (not (`self.IsDown`))
      (`BlackboardComponent.SetValueAsVector` _returnvalue (`self.HearLocation`) Location)
      (`BlackboardComponent.SetValueAsBool` _returnvalue (`self.IsHeared`) true))))

(event `self.PawnSensing.OnSeePawn`
  (params (Pawn :type "Pawn Object Reference"))
  ;[1 1 1] SeePlayer
  (if (`KismetSystemLibrary.IsServer`)
    (`BlackboardComponent.SetValueAsObject` (`AIBlueprintHelperLibrary.GetBlackboard` self) (`self.Player`) Pawn)))

(event `FaceToPlayer`
  (params (Player :type "Actor Object Reference"))
  ;[1 1 1] FaseToPlayer
  (bind _returnvalue (`self.ActorLookAtPoint` Player))
  (bind _output_get (set `self.LookAtPoint` _returnvalue))
  (`self.K2_SetActorRotation` (`KismetMathLibrary.FindLookAtRotation` (`self.K2_GetActorLocation`) _output_get)))

(event `MoveTo`
  (params (Target :type "Vector Structure"))
  ;[1 1 1] MoveTo
  (`AIBlueprintHelperLibrary.SimpleMoveToLocation` (`AIBlueprintHelperLibrary.GetAIController` self) Target))

(event `ROM_RunSucceed`
  (bind _weaponslot_weaponbase (break `/Game/ShootingRange/Blueprints/Weapons/SWeaponSlot` (`self.WeaponSlot`)))
  (bind _skeletalmesh (`/Game/ShootingRange/Blueprints/Weapons/BP_WeaponBase.SkeletalMesh` _weaponslot_weaponbase))
  ;[1 1 1] RunAwaySucceed
  (`self.DetachFromControllerPendingDestroy`)
  (`MovementComponent.StopMovementImmediately` (`self.CharacterMovement`))
  (`self.SetLifeSpan` 1.0)
  (`PrimitiveComponent.SetSimulatePhysics` _skeletalmesh true)
  (`PrimitiveComponent.SetCollisionResponseToChannel` _skeletalmesh "ECC_GameTraceChannel1" "ECR_Block"))

(event `ROM_SetHpBar`
  (params (HpPersant :type "Float (double-precision)"))
  ;[1 1 1] UpdateHPBar
  (message `/Game/ShootingRange/UI/WBPI_HpBar.SendHp` (`WidgetComponent.GetWidget` (`self.Widget`)) HpPersant))

(fn `ActorLookAtPoint`
  (params (Player :type "Actor Object Reference"))
  (returns (ReturnValue :type "Vector Structure"))
  (bind _returnvalue_location (`KismetMathLibrary.BreakTransform` (`SceneComponent.GetSocketTransform` (`self.Mesh`) "head" "RTS_World")))
  (bind (_outhit _returnvalue) (`KismetSystemLibrary.LineTraceSingle` :`Start` _returnvalue_location :`End` (`self.K2_GetActorLocation` Player) :`TraceChannel` "TraceTypeQuery1" :`DrawDebugType` "ForOneFrame"))
  (bind (_bblockinghit _binitialoverlap _time _distance _location _impactpoint _normal _impactnormal _physmat _hitactor _hitcomponent _hitbonename _hititem _faceindex _tracestart _traceend) (`GameplayStatics.BreakHitResult` _outhit))
  (return (`KismetMathLibrary.SelectVector` _location _traceend _returnvalue)))

(fn `CaculateLHandOfset`
  (bind _weaponslot_weaponbase (break `/Game/ShootingRange/Blueprints/Weapons/SWeaponSlot` (`self.WeaponSlot`)))
  (bind _returnvalue_location (`KismetMathLibrary.BreakTransform` (`SceneComponent.GetSocketTransform` (`/Game/ShootingRange/Blueprints/Weapons/BP_WeaponBase.SkeletalMesh` _weaponslot_weaponbase) "GripL" "RTS_World")))
  (`/Engine/EditorBlueprintResources/StandardMacros.IsValid` _weaponslot_weaponbase
    (:`Is Valid`
      (set `self.GripLOfset` (`SkinnedMeshComponent.TransformToBoneSpace` :`self` (`self.Mesh`) :`BoneName` "hand_r" :`InPosition` _returnvalue_location)))))

(fn `EnemySendValue`
  (returns (Values :type "/Game/ShootingRange/Blueprints/Character/BPIS_SendValue Structure"))
  (return (make `/Game/ShootingRange/Blueprints/Character/BPIS_SendValue` (`self.Yaw`) (`self.Pitch`) (`self.Dirction`) (`self.Speed`) (`self.IsInAir`) (`self.IsCombate`) (`self.IsADS`) (`self.UseLHandIK`) (`self.GripLOfset`) (`self.Aim Baseline Offset`) (`self.Weapon Type`))))

(fn `LossWeapon`
  (bind _weaponslot_weaponbase (break `/Game/ShootingRange/Blueprints/Weapons/SWeaponSlot` (`self.WeaponSlot`)))
  (bind _skeletalmesh (`/Game/ShootingRange/Blueprints/Weapons/BP_WeaponBase.SkeletalMesh` _weaponslot_weaponbase))
  (`PrimitiveComponent.SetSimulatePhysics` _skeletalmesh true)
  (`PrimitiveComponent.SetCollisionResponseToChannel` _skeletalmesh "ECC_GameTraceChannel1" "ECR_Block"))

(fn `ToggleHandL IK`
  (bind (_weaponslot_weaponbase _weaponslot_weapontype) (break `/Game/ShootingRange/Blueprints/Weapons/SWeaponSlot` (`self.WeaponSlot`)))
  (set `self.UseLHandIK` (and (!= _weaponslot_weaponbase null) (`|EnumEquality` _weaponslot_weapontype "NewEnumerator0") (`self.IsCombate`) (== (`AnimInstance.GetCurveValue` (`SkeletalMeshComponent.GetAnimInstance` (`self.Mesh`)) "HandL IK Off") 0.0) (not (`self.IsDown`)))))

(fn `UserConstructionScript`)