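; BP_ProjectileBase is a projectile actor, by name the base for shooting-range weapons, that deals damage and pushes physics objects on impact.
; When its StaticMesh hits a valid component, the server applies damage, crediting player pawn 0 as causer.
; If that component simulates physics, the ROM_ApplyImpose event adds an impulse at the hit point along the projectile's forward vector.
; The projectile destroys itself on every hit, on server or client.
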(event `self.StaticMesh.OnComponentHit`
  (params (HitComponent :type "PrimitiveComponent Object Reference") (OtherActor :type "Actor Object Reference") (OtherComp :type "PrimitiveComponent Object Reference") (NormalImpulse :type "Vector Structure") (Hit :type "HitResult Structure (by ref)"))
  (bind (_bblockinghit _binitialoverlap _time _distance _location _impactpoint _normal _impactnormal _physmat _hitactor _hitcomponent) (`GameplayStatics.BreakHitResult` Hit))
  (if (`KismetSystemLibrary.IsServer`)
    (if (`KismetSystemLibrary.IsValid` _hitcomponent)
      (`GameplayStatics.ApplyDamage` OtherActor (`self.Damage`) null (`GameplayStatics.GetPlayerPawn` 0))
      (if (`SceneComponent.IsSimulatingPhysics` _hitcomponent "None")
        (`self.ROM_ApplyImpose` _hitcomponent (* (`KismetMathLibrary.GetForwardVector` (`self.K2_GetActorRotation` self)) (`self.Impulse`)) _location))
      (`self.K2_DestroyActor`)
      (else
        (`self.K2_DestroyActor`)))
    (else
      (`self.K2_DestroyActor`))))

(event `ROM_ApplyImpose`
  (params (`目标` :type "PrimitiveComponent Object Reference") (Impulse :type "Vector Structure") (Location :type "Vector Structure"))
  (`PrimitiveComponent.AddImpulseAtLocation` `目标` Impulse Location "None"))

(fn `UserConstructionScript`)