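; Base weapon actor for BP_MyCharacter and BP_Enemy, handling firing, reloading, fire-mode switching and a toggleable light.
; Fire branches into single, burst (Semi-Auto), looping full-auto or shotgun spread (My Gun), spawning BP_ProjectileBase at the muzzle.
; Shots aim at the owner's look-at point, or along the muzzle when absolute yaw reaches 90 degrees.
; ROM events play montages and sounds, with server-only MakeNoise calls.
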(event `ROS_GetWeapon`
  (params (Object :type "Object Object Reference"))
  ;[1 1 1] GetWeaponOnwer
  (bind _asbp_my_character (cast `/Game/ShootingRange/Blueprints/Character/BP_MyCharacter` Object)
    (:`then`
      (set `self.Owning Character` _asbp_my_character)
      (set `self.IsCharacter` true))
    (:`CastFailed`
      (bind _asbp_enemy (cast `/Game/ShootingRange/Blueprints/Enemy/BP_Enemy` Object))
      (set `self.Owning Enemy` _asbp_enemy)
      (set `self.IsCharacter` false)))
  (set `self.AimBaselineOffset` (- (`KismetAnimationLibrary.K2_DistanceBetweenTwoSocketsAndMapRange` (`self.SkeletalMesh`) "Root" "RTS_World" "Sight" "RTS_World") 13.53))
  (set `self.RoundsInChamber` (`self.MagSize`)))

(event `/Game/ShootingRange/Blueprints/Weapons/BPI_WeaponBase.GetWeapon`
  (params (OwningCharacter :type "Actor Object Reference"))
  ;[1 1 1] GetWeaponOnwer
  (`self.ROS_GetWeapon` OwningCharacter))

(event `ToggleFireModeWeapon`
  ;[1 1 1] ToggleFireMode
  (if (> (`KismetArrayLibrary.Array_Length` (`self.AvailableFireMode`)) 1)
    (bind _nextitem (`/Game/ShootingRange/Blueprints/Character/BPML_MacroLibrary.GetArrayNextItem` (`self.AvailableFireMode`) (`self.FireMode`))
      (:`Out`
        (set `self.FireMode` _nextitem)
        (`self.ROM_ToggleFireMode`)))))

(event `ROM_ToggleFireMode`
  (bind _returnvalue (`self.K2_GetActorLocation`))
  ;[1 1 1] ToggleFireMode
  (`GameplayStatics.PlaySoundAtLocation` "/Game/ShootingRange/Audio/换切开火.换切开火" _returnvalue (struct) 1.0 1.0 0.0 null null null)
  (if (`KismetSystemLibrary.IsServer`)
    (`self.MakeNoise` 1.0 (`self.Owning Character`) _returnvalue)))

(event `ReloadWeapon`
  ;[1 1 1] Reload
  (set `self.RoundsInChamber` (`self.MagSize`))
  (`self.ROM_Reload` (`self.SkeletalMesh`) (`self.ReloadMontageWeapon`) (`self.ReloadSound`)))

(event `ROM_Reload`
  (params (InSkeletalMeshComponent :type "SkeletalMeshComponent Object Reference") (MontageToPlay :type "AnimMontage Object Reference") (Sound :type "SoundBase Object Reference"))
  (bind _returnvalue (`self.K2_GetActorLocation`))
  ;[1 1 1] Reload
  (`|PlayMontage` InSkeletalMeshComponent MontageToPlay
    (:`then`
      (`GameplayStatics.PlaySoundAtLocation` Sound _returnvalue (struct) 1.0 1.0 0.0 null null null)
      (if (`KismetSystemLibrary.IsServer`)
        (`self.MakeNoise` 1.0 (`self.Owning Character`) _returnvalue)))))

(event `OpenLight`
  (params (OpenLight :type Boolean))
  (bind _spotlight (`self.SpotLight`))
  ;[1 1 1] OpenWeaponLight
  (if OpenLight
    (`LightComponent.SetIntensity` _spotlight (`self.LightIntensity`))
    (else
      (`LightComponent.SetIntensity` _spotlight 0.0))))

(event `/Game/ShootingRange/Blueprints/Weapons/BPI_WeaponBase.FireWeapon`
  ;[1 1 1] Fire
  (if (> (`self.RoundsInChamber`) 0)
    (set `self.IsFiring` true)
    (`self.Fire`)
    (else
      (`self.ROM_NoBulletSound`))))

(event `ROM_NoBulletSound`
  (bind _returnvalue (`self.K2_GetActorLocation`))
  ;[1 1 1] Fire
  (`GameplayStatics.PlaySoundAtLocation` "/Game/ShootingRange/Audio/空膛.空膛" _returnvalue (struct) 1.0 1.0 0.0 null null null)
  (if (`KismetSystemLibrary.IsServer`)
    (`self.MakeNoise` 1.0 (`self.Owning Character`) _returnvalue)))

(event `RepeatFire`
  (bind (_shotgunrandomcircle_x _shotgunrandomcircle_y) (`KismetMathLibrary.BreakVector2D` (`self.ShotGunRandomCircle`)))
  (bind _returnvalue (`KismetMathLibrary.SelectVector` (`KismetMathLibrary.GetForwardVector` (`SceneComponent.GetSocketRotation` (`self.SkeletalMesh`) "Muzzle")) (- (`self.GetOwnerLookAtPoint`) (`SceneComponent.GetSocketLocation` (`self.SkeletalMesh`) "Muzzle")) (>= (`KismetMathLibrary.Abs` (`self.GetOwnerYaw`)) 90.0)))
  ;[1 1 1] Fire
  (switch `/Game/ShootingRange/Blueprints/Weapons/EFireMode` (`self.FireMode`) :!label _label
    (:`NewEnumerator0`
      (`/Engine/EditorBlueprintResources/StandardMacros.DoOnce` false :!label _label_2
        (:`Completed`
          (`self.ROM_FireMontage` (`self.GetOwnerMesh`) (/ (`self.RBM`) 200.0) (`self.FireSound`) (`self.SkeletalMesh`) (`self.FireMontageWeapon`))
          (`|ExecutionSequence`
            (:`then_0`
              (`KismetSystemLibrary.Delay` 0.3)
              (goto _label_2 :!via `Reset`))
            (:`then_1`
              (bind _returnvalue_2 (`|SpawnActorFromClass` "/Game/ShootingRange/Blueprints/Weapons/BP_ProjectileBase.BP_ProjectileBase_C" (`SceneComponent.GetSocketTransform` (`self.SkeletalMesh`) "Muzzle" "RTS_World") "AlwaysSpawn" "OverrideRootScale" null null :!label _label_3))
              (set `MovementComponent.Velocity` (* (`KismetMathLibrary.Normal` (`KismetMathLibrary.SelectVector` (`KismetMathLibrary.GetForwardVector` (`SceneComponent.GetSocketRotation` (`self.SkeletalMesh`) "Muzzle")) (- (`self.GetOwnerLookAtPoint`) (`SceneComponent.GetSocketLocation` (`self.SkeletalMesh`) "Muzzle")) (>= (`KismetMathLibrary.Abs` (`self.GetOwnerYaw`)) 90.0))) (`self.MuzzleVelocity`)) (`/Game/ShootingRange/Blueprints/Weapons/BP_ProjectileBase.ProjectileMovement` _returnvalue_2))
              (`/Engine/EditorBlueprintResources/StandardMacros.DecrementInt` (`self.RoundsInChamber`)))))))
    (:`NewEnumerator2`
      (`self.ROM_FireMontage` (`self.GetOwnerMesh`) (/ (`self.RBM`) 200.0) (`self.FireSound`) (`self.SkeletalMesh`) (`self.FireMontageWeapon`))
      (`|ExecutionSequence`
        (:`then_0`
          (`KismetSystemLibrary.Delay` 0.2)
          (`/Engine/EditorBlueprintResources/StandardMacros.IncrementInt` (`self.FireNum`)
            (:`  `
              (`self.ShouldRepeatCheckSemiAuto`))))
        (:`then_1`
          (goto _label_3))))
    (:`NewEnumerator3`
      (`self.ROM_FireMontage` (`self.GetOwnerMesh`) (/ (`self.RBM`) 200.0) (`self.FireSound`) (`self.SkeletalMesh`) (`self.FireMontageWeapon`))
      (`|ExecutionSequence`
        (:`then_0`
          (`KismetSystemLibrary.Delay` 0.2)
          (`self.ShouldRepeatCheckFullAuto`))
        (:`then_1`
          (goto _label_3))))
    (:`NewEnumerator4`
      (`/Engine/EditorBlueprintResources/StandardMacros.DoOnce` false :!label _label_4
        (:`Completed`
          (`/Engine/EditorBlueprintResources/StandardMacros.DecrementInt` (`self.RoundsInChamber`)
            (:`  `
              (`self.ROM_FireMontageWithoutWeapon` (`self.GetOwnerMesh`) (/ (`self.RBM`) 200.0) (`self.FireSound`))
              (for _ (range 1 (+ (`self.ShotGunBurstNum`) 1))
                (set `self.ShotGunDistance` (`KismetMathLibrary.VSize` _returnvalue))
                (bind _point (`self.RandPointInCircle` (* (`KismetMathLibrary.DegTan` (`self.ShotGunBulletAngle`)) (`self.ShotGunDistance`))))
                (set `self.ShotGunRandomCircle` _point)
                (bind _returnvalue_3 (`|SpawnActorFromClass` "/Game/ShootingRange/Blueprints/Weapons/BP_ProjectileBase.BP_ProjectileBase_C" (`SceneComponent.GetSocketTransform` (`self.SkeletalMesh`) "Muzzle" "RTS_World") "AlwaysSpawn" "OverrideRootScale" null null))
                (set `MovementComponent.Velocity` (* (`KismetMathLibrary.Normal` (`KismetMathLibrary.MakeVector` (+ _shotgunrandomcircle_x (.x _returnvalue)) (+ _shotgunrandomcircle_y (.y _returnvalue)) (.z _returnvalue))) (`self.MuzzleVelocity`)) (`/Game/ShootingRange/Blueprints/Weapons/BP_ProjectileBase.ProjectileMovement` _returnvalue_3)))
              (`KismetSystemLibrary.Delay` 0.4)
              (goto _label_4 :!via `Reset`))))))))

(event `FireRelease`
  ;[1 1 1] Fire
  ;;[1 1 1] ReleaseFire
  (set `self.IsFiring` false))

(event `Fire`
  ;[1 1 1] Fire
  (goto _label))

(event `ROM_FireMontageWithoutWeapon`
  (params (CharacterMesh :type "SkeletalMeshComponent Object Reference") (PlayRate :type "Float (double-precision)") (Sound :type "SoundBase Object Reference"))
  (bind _returnvalue (`self.K2_GetActorLocation`))
  ;[1 1 1] Fire
  (`|PlayMontage` CharacterMesh "/Game/ShootingRange/Assets/Character/Animations/AM_2HW_ADS_Fire.AM_2HW_ADS_Fire" PlayRate
    (:`OnNotifyBegin`
      (`GameplayStatics.PlaySoundAtLocation` Sound _returnvalue (struct) 1.0 1.0 0.0 null null null)
      (if (`KismetSystemLibrary.IsServer`)
        (`self.MakeNoise` 1.0 (`self.Owning Character`) _returnvalue)))))

(event `ROM_FireMontage`
  (params (CharacterMesh :type "SkeletalMeshComponent Object Reference") (PlayRate :type "Float (double-precision)") (Sound :type "SoundBase Object Reference") (WeaponMesh :type "SkeletalMeshComponent Object Reference") (MontageToPlay :type "AnimMontage Object Reference"))
  (bind _returnvalue (`self.K2_GetActorLocation`))
  ;[1 1 1] Fire
  (`|PlayMontage` CharacterMesh "/Game/ShootingRange/Assets/Character/Animations/AM_2HW_ADS_Fire.AM_2HW_ADS_Fire" PlayRate
    (:`then`
      (`|PlayMontage` WeaponMesh MontageToPlay PlayRate))
    (:`OnNotifyBegin`
      (`GameplayStatics.PlaySoundAtLocation` Sound _returnvalue (struct) 1.0 1.0 0.0 null null null)
      (if (`KismetSystemLibrary.IsServer`)
        (`self.MakeNoise` 1.0 (`self.Owning Character`) _returnvalue)))))

(fn `GetOwnerLookAtPoint`
  (returns (ReturnValue :type "Vector Structure"))
  (return (select `bool` (`self.IsCharacter`) :`false` (`/Game/ShootingRange/Blueprints/Enemy/BP_Enemy.LookAtPoint` (`self.Owning Enemy`)) :`true` (`/Game/ShootingRange/Blueprints/Character/BP_MyCharacter.LookAtPoint` (`self.Owning Character`)))))

(fn `GetOwnerMesh`
  (returns (ReturnValue :type "SkeletalMeshComponent Object Reference"))
  (return (select `bool` (`self.IsCharacter`) :`false` (`Character.Mesh` (`self.Owning Enemy`)) :`true` (`Character.Mesh` (`self.Owning Character`)))))

(fn `GetOwnerYaw`
  (returns (ReturnValue :type "Float (double-precision)"))
  (return (select `bool` (`self.IsCharacter`) :`false` (`/Game/ShootingRange/Blueprints/Enemy/BP_Enemy.Yaw` (`self.Owning Enemy`)) :`true` (`/Game/ShootingRange/Blueprints/Character/BP_MyCharacter.Yaw` (`self.Owning Character`)))))

(fn `GetWeaponPanelInfo`
  (returns (WeaponBase :type "/Game/ShootingRange/Blueprints/Weapons/BP_WeaponBase Object Reference") (WeaponType :type "/Game/ShootingRange/Blueprints/Weapons/EWeaponType Enum"))
  (return self (`self.WeaponType`)))

(fn `RandPointInCircle`
  (params (Radius :type "Float (double-precision)"))
  (returns (Point :type "Vector2D Structure"))
  (locals (Angle :type "Float (double-precision)") (DistanceFromCenter :type "Float (double-precision)"))
  (bind _distancefromcenter (`local.DistanceFromCenter`))
  (set `local.DistanceFromCenter` (`KismetMathLibrary.RandomFloatInRange` 0.0 Radius))
  (set `local.Angle` (`KismetMathLibrary.RandomFloatInRange` 0.0 360.0))
  (return (`KismetMathLibrary.MakeVector2D` (* _distancefromcenter (`KismetMathLibrary.DegCos` (`local.Angle`))) (* (`KismetMathLibrary.DegSin` (`local.Angle`)) _distancefromcenter))))

(fn `SendValue`
  (returns (WeaponValue :type "/Game/ShootingRange/Blueprints/Weapons/SWeaponSendValue Structure"))
  (return (make `/Game/ShootingRange/Blueprints/Weapons/SWeaponSendValue` (`self.WeaponName`) (`self.FireMode`) (`self.RoundsInChamber`) (`self.MagSize`))))

(fn `ShouldRepeatCheckFullAuto`
  (bind _returnvalue (`self.K2_GetActorLocation`))
  (bind _isfiring (`self.IsFiring`))
  (if (and _isfiring (> (`self.RoundsInChamber`) 0))
    (`self.RepeatFire`)
    (elif _isfiring
      (`GameplayStatics.PlaySoundAtLocation` "/Game/ShootingRange/Audio/空膛.空膛" _returnvalue (struct) 1.0 1.0 0.0 null null null)
      (if (`KismetSystemLibrary.IsServer`)
        (`self.MakeNoise` 1.0 (`self.Owning Character`) _returnvalue)))))

(fn `ShouldRepeatCheckSemiAuto`
  (bind _returnvalue (`self.K2_GetActorLocation`))
  (bind _returnvalue_2 (< (`self.FireNum`) (`self.SimeFireNum`)))
  (if (and (> (`self.RoundsInChamber`) 0) _returnvalue_2)
    (`self.RepeatFire`)
    (else
      (if _returnvalue_2
        (`GameplayStatics.PlaySoundAtLocation` "/Game/ShootingRange/Audio/空膛.空膛" _returnvalue (struct) 1.0 1.0 0.0 null null null))
      (set `self.FireNum` 0)
      (if (`KismetSystemLibrary.IsServer`)
        (`self.MakeNoise` 1.0 (`self.Owning Character`) _returnvalue)))))

(fn `UserConstructionScript`)