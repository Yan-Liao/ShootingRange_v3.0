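; Thrown grenade for the shooting range that explodes 1.5 seconds after ThrowedGrenade fires.
; The blast plays sound and particles, makes noise attributed to player pawn 0, hides the mesh and sets a short lifespan.
; A debug-drawn sphere trace then damages PhysicsBody hits and pushes simulating components away from the center.
; Effects and impulses run through separate ROM_ events.
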(event `ROM_GrenadeBoom`
  (params (Location :type "Vector Structure"))
  (`GameplayStatics.PlaySoundAtLocation` "/Game/ShootingRange/Audio/手雷爆炸.手雷爆炸" Location (struct) 1.0 1.0 0.0 null null null)
  (`self.MakeNoise` 1.0 (`GameplayStatics.GetPlayerPawn` 0) Location)
  (`GameplayStatics.SpawnEmitterAtLocation` "/Game/FXVarietyPack/P_ky_explosion.P_ky_explosion" Location)
  (`SceneComponent.SetHiddenInGame` (`self.StaticMesh`) true false)
  (`self.SetLifeSpan` 2.0))

(event `ROM_ApplyImplse`
  (params (HitComponet :type "PrimitiveComponent Object Reference") (Impulse :type "Vector Structure") (Location :type "Vector Structure"))
  (`PrimitiveComponent.AddImpulseAtLocation` HitComponet Impulse Location "None"))

(event `ThrowedGrenade`
  (bind _returnvalue (`SceneComponent.K2_GetComponentLocation` (`self.StaticMesh`)))
  (`KismetSystemLibrary.Delay` 1.5)
  (`self.ROM_GrenadeBoom` _returnvalue)
  (bind (_outhits _returnvalue_2) (`KismetSystemLibrary.SphereTraceMultiForObjects` :`Start` _returnvalue :`End` _returnvalue :`Radius` 350.0 :`ObjectTypes` (`|MakeArray` "ObjectTypeQuery4" :!type "EObjectTypeQuery Enum") :`DrawDebugType` "ForDuration"))
  (if _returnvalue_2
    (for _array_element _outhits
      (bind (_bblockinghit _binitialoverlap _time _distance _location _impactpoint _normal _impactnormal _physmat _hitactor _hitcomponent) (`GameplayStatics.BreakHitResult` _array_element))
      (`GameplayStatics.ApplyDamage` _hitactor (`self.Damege`))
      (if (`SceneComponent.IsSimulatingPhysics` _hitcomponent "None")
        (`self.ROM_ApplyImplse` _hitcomponent (* (`KismetMathLibrary.GetDirectionUnitVector` (`SceneComponent.K2_GetComponentLocation` (`self.StaticMesh`)) (`SceneComponent.K2_GetComponentLocation` _hitcomponent)) (`self.Impulse`)) _location)))))

(fn `UserConstructionScript`)