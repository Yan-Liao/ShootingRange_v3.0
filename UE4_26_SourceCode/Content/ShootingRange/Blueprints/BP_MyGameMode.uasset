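; Game mode for the ShootingRange game that handles multiplayer match start, map change and session teardown.
; It records each player controller on login.
; Starting a game has each BP_MyPlayerController create a loading UI, then changes map through a console command built from the map name.
; When the server leaves, it destroys the session for every listed player.
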(event `self.K2_OnSwapPlayerControllers`
  (params (OldPC :type "PlayerController Object Reference") (NewPC :type "PlayerController Object Reference")))

(event `self.K2_PostLogin`
  (params (NewPlayer :type "PlayerController Object Reference"))
  ;[1 1 1] 玩家登录时
  (`KismetArrayLibrary.Array_AddUnique` (`self.PlayerList`) NewPlayer))

(event `ROS_StartGame`
  (params (MapName :type String))
  ;[1 1 1] 服务器将开始游戏的信息传给客户端
  (for _array_element (`self.PlayerList`)
    (bind _asbp_my_player_controller (cast `/Game/ShootingRange/Blueprints/BP_MyPlayerController` _array_element))
    (`/Game/ShootingRange/Blueprints/BP_MyPlayerController.ROC_CreateLoadingUI` _asbp_my_player_controller _asbp_my_player_controller))
  (`self.ROS_JumpToMap` MapName))

(event `ROS_JumpToMap`
  (params (MapName :type String))
  ;[1 1 1] 跳到指定关卡
  (`KismetSystemLibrary.ExecuteConsoleCommand` (`KismetStringLibrary.Concat_StrStr` (`self.Command1`) MapName) (`GameplayStatics.GetPlayerController` 0)))

(event `ROS_ServerLeave`
  ;[1 1 1] ServerLeave
  (for _array_element (`self.PlayerList`)
    (`self.ROM_ClearSession` _array_element)))

(event `ROM_ClearSession`
  (params (PlayerController :type "PlayerController Object Reference"))
  ;[1 1 1] ServerLeave
  (`DestroySessionCallbackProxy.DestroySession` PlayerController))

(fn `UserConstructionScript`)