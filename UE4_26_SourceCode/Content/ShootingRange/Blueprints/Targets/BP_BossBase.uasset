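; Base boss target for the multiplayer shooting range: an AI enemy that pursues and attacks players.
; BossDebut sets up the blackboard with the nearest player and notifies its controller, with movement, attack and retargeting exposed as events.
; Damage updates a widget health bar; at zero HP it detaches the controller, drops the plane with physics and notifies GameState.
; ROS/ROM events separate server logic from multicast feedback, while the periodic retargeting timer is left unwired.
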(event `self.ReceiveBeginPlay`
  (`self.ROS_Init`))

(event `ROS_Init`
  (set `self.Hp` (`self.MaxHp`)))

(event `ROM_HitSound`
  ;[1 1 1] GetDamage
  (`AudioComponent.Play` (`self.ACBeHit`) 0.0))

(event `ROS_BossDebut`
  ;[1 1 1] BossDebut
  (`self.SetBlackBoard`)
  (bind _asbp_boss_controler (cast `/Game/ShootingRange/Blueprints/Targets/AI/BP_BossControler` (`self.GetController` self)))
  (`/Game/ShootingRange/Blueprints/Targets/AI/BP_BossControler.BossComing` _asbp_boss_controler)
  (`self.ROM_BossDebutSound`))

(event `/Game/ShootingRange/Blueprints/Targets/BPI_Boss.BossDebut`
  ;[1 1 1] BossDebut
  (`self.ROS_BossDebut`))

(event `ROM_BossDebutSound`
  ;[1 1 1] BossDebut
  (`AudioComponent.Play` (`self.ACTargetUp`) 0.0))

(event `self.ReceiveAnyDamage`
  (params (Damage :type "Float (single-precision)") (DamageType :type "DamageType Object Reference") (InstigatedBy :type "Controller Object Reference") (DamageCauser :type "Actor Object Reference"))
  ;[1 1 1] GetDamage
  (`|ExecutionSequence`
    (:`then_0`
      (`self.ROM_HitSound`))
    (:`then_1`
      (if (not (`self.TargetIsDown`))
        (bind _output_get (set `self.Hp` (`KismetMathLibrary.FMax` (- (`self.Hp`) Damage))))
        (`|ExecutionSequence`
          (:`then_0`
            (`/Engine/EditorBlueprintResources/StandardMacros.CompareFloat` _output_get
              (:`==`
                _)
              (:`<`
                _))
            (`/Engine/EditorBlueprintResources/StandardMacros.DoOnce` false
              (:`Completed`
                (set `self.TargetIsDown` true)
                (`KismetSystemLibrary.K2_ClearTimer` null "ChoosePlayer")
                (`self.ROM_BossDown`))))
          (:`then_1`
            (`self.ROM_SetHpBar` (/ (`self.Hp`) (`self.MaxHp`)))))))))

(event `ROM_BossDown`
  ;[1 1 1] GetDamage
  (`self.DetachFromControllerPendingDestroy`)
  (`SceneComponent.SetHiddenInGame` (`self.Widget`) true false)
  (`PrimitiveComponent.SetSimulatePhysics` (`self.Shape_Plane`) true)
  (`PrimitiveComponent.SetConstraintMode` (`self.Shape_Plane`) "None")
  (`AudioComponent.Play` (`self.ACTargetDown`) 0.0)
  (bind _asbp_my_game_state (cast `/Game/ShootingRange/Blueprints/BP_MyGameState` (`GameplayStatics.GetGameState`)))
  (`/Game/ShootingRange/Blueprints/BP_MyGameState.EnemyDown` _asbp_my_game_state))

(event `/Game/ShootingRange/Blueprints/Targets/BPI_Boss.Attack`
  (params (AttackWho :type "Actor Object Reference"))
  ;[1 1 1] ApplyDamage
  (`GameplayStatics.ApplyDamage` AttackWho (`self.Damage`) null self)
  (`self.ROM_AttackSound`))

(event `ROM_AttackSound`
  ;[1 1 1] ApplyDamage
  (`AudioComponent.Play` (`self.ACHit`) 0.0))

(event `SetBlackBoard`
  (bind _returnvalue (`AIBlueprintHelperLibrary.GetBlackboard` self))
  ;[1 1 1] 初始化设置黑板
  (if (`KismetSystemLibrary.IsServer`)
    (`AIController.UseBlackboard` (`AIBlueprintHelperLibrary.GetAIController` self) "/Game/ShootingRange/Blueprints/Targets/AI/BB_Boss.BB_Boss")
    (bind _returnvalue_2 (`self.GetClosePlayer`))
    (`BlackboardComponent.SetValueAsObject` _returnvalue (`self.FindWho`) _returnvalue_2)
    (`BlackboardComponent.SetValueAsObject` _returnvalue (`self.SelfName`) self)))

(event `/Game/ShootingRange/Blueprints/Targets/BPI_Boss.MoveTo`
  (params (Target :type "Actor Object Reference"))
  ;[1 1 1] MoveTo
  (if (not (`self.TargetIsDown`))
    (`AIBlueprintHelperLibrary.SimpleMoveToActor` (`AIBlueprintHelperLibrary.GetAIController` self) Target)))

(event `ChoosePlayer`
  ;[1 1 1] ChooseClosePlayer
  (if (not (`self.TargetIsDown`))
    (bind _returnvalue (`self.GetClosePlayer`))
    (`BlackboardComponent.SetValueAsObject` (`AIBlueprintHelperLibrary.GetBlackboard` self) (`self.FindWho`) _returnvalue)))

(event `ROM_SetHpBar`
  (params (HpPersant :type "Float (double-precision)"))
  ;[1 1 1] UpdateHPBar
  (message `/Game/ShootingRange/UI/WBPI_HpBar.SendHp` (`WidgetComponent.GetWidget` (`self.Widget`)) HpPersant))

(event `/Game/ShootingRange/Blueprints/Targets/BPI_Boss.PlayerDown`
  (`self.DetachFromControllerPendingDestroy`))

(fn `GetClosePlayer`
  (returns (ReturnValue :type "Pawn Object Reference"))
  (locals (MinDistance :type "Float (double-precision)") (ClosePlayerIndex :type Integer))
  (bind _asbp_my_game_mode (cast `/Game/ShootingRange/Blueprints/BP_MyGameMode` (`GameplayStatics.GetGameMode`)))
  (bind _playerlist (`/Game/ShootingRange/Blueprints/BP_MyGameMode.PlayerList` _asbp_my_game_mode))
  (set `local.MinDistance` (`self.GetDistanceTo` (`Controller.K2_GetPawn` (`|GetArrayItem` _playerlist (`local.ClosePlayerIndex`))) self))
  (for (_array_element _array_index) _playerlist
    (bind _returnvalue (`self.GetDistanceTo` (`Controller.K2_GetPawn` _array_element) self))
    (`/Engine/EditorBlueprintResources/StandardMacros.CompareFloat` _returnvalue (`local.MinDistance`)
      (:`<`
        (set `local.MinDistance` _returnvalue)
        (set `local.ClosePlayerIndex` _array_index))))
  (return (`Controller.K2_GetPawn` (`|GetArrayItem` _playerlist (`local.ClosePlayerIndex`)))))

(fn `UserConstructionScript`)