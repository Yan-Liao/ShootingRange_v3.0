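; Hostage target for the shooting range that the player must save without shooting it, deciding mission success or failure.
; Saving, when allowed, runs once, swaps the plane's material, removes its box and reports success to the game state.
; Damage plays hit audio or feedback and drains health; at zero the plane's constraint mode is cleared and failure is reported after a delay.
; A tip trigger shows and removes the save-prompt widget on overlap.
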(event `ROM_Saved`
  (`PrimitiveComponent.SetMaterial` (`self.Shape_Plane`) 0 "/Game/ShootingRange/Assets/Target/M_Hostage2.M_Hostage2")
  (`ActorComponent.K2_DestroyComponent` (`self.Box`))
  (message `/Game/ShootingRange/Blueprints/BPI_MyGameState.MissionSucceed` (`GameplayStatics.GetGameState`)))

(event `saving`
  (if (`self.CanBeSaved`)
    (`/Engine/EditorBlueprintResources/StandardMacros.DoOnce` false
      (:`Completed`
        (`self.ROM_Saved`)
        (set `self.IsSaved` true)))))

(event `self.ReceiveAnyDamage`
  (params (Damage :type "Float (single-precision)") (DamageType :type "DamageType Object Reference") (InstigatedBy :type "Controller Object Reference") (DamageCauser :type "Actor Object Reference"))
  (`|ExecutionSequence`
    (:`then_0`
      (`AudioComponent.Play` (`self.ACBeHit`) 0.0))
    (:`then_1`
      (if (not (`self.TargetIsDown`))
        (bind _output_get (set `self.TargetHp` (`KismetMathLibrary.FMax` (- (`self.TargetHp`) Damage))))
        (`/Engine/EditorBlueprintResources/StandardMacros.CompareFloat` _output_get
          (:`==`
            _)
          (:`<`
            _))
        (`/Engine/EditorBlueprintResources/StandardMacros.DoOnce` false
          (:`Completed`
            (set `self.TargetIsDown` true)
            (`PrimitiveComponent.SetConstraintMode` (`self.Shape_Plane`) "None")
            (`KismetSystemLibrary.Delay` 1.0)
            (message `/Game/ShootingRange/Blueprints/BPI_MyGameState.MissionFailed` (`GameplayStatics.GetGameState`) "NewEnumerator2")))))))

(event `self.Tip.OnComponentBeginOverlap`
  (params (OverlappedComponent :type "PrimitiveComponent Object Reference") (OtherActor :type "Actor Object Reference") (OtherComp :type "PrimitiveComponent Object Reference") (OtherBodyIndex :type Integer) (bFromSweep :type Boolean) (SweepResult :type "HitResult Structure (by ref)"))
  (`/Engine/EditorBlueprintResources/StandardMacros.DoOnce` false :!label _label
    (:`Completed`
      (bind _returnvalue (`|CreateWidget` "/Game/ShootingRange/UI/WBP_Tip5.WBP_Tip5_C"))
      (bind _output_get (set `self.UI SaveTip` _returnvalue))
      (`UserWidget.AddToViewport` _output_get 0))))

(event `self.Tip.OnComponentEndOverlap`
  (params (OverlappedComponent :type "PrimitiveComponent Object Reference") (OtherActor :type "Actor Object Reference") (OtherComp :type "PrimitiveComponent Object Reference") (OtherBodyIndex :type Integer))
  (`|ExecutionSequence`
    (:`then_0`
      (goto _label :!via `Reset`))
    (:`then_1`
      (`Widget.RemoveFromParent` (`self.UI SaveTip`)))))

(fn `UserConstructionScript`)